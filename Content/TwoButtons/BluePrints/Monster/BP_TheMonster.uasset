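; BP_TheMonster is an AI-driven monster that becomes alerted when it spots the player.
; Its PawnSensing component reacts to the first sighted pawn tagged Player, latching an Alerted flag that this Blueprint never clears.
; That sighting writes the alert state and target pawn to the AI controller's Blackboard and swaps the HeavyBreathing sound to an alerted one.
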(event `self.ReceiveBeginPlay`)

(event `self.ReceiveActorBeginOverlap`
  (params (OtherActor :type "Actor Object Reference")))

(event `self.ReceiveTick`
  (params (DeltaSeconds :type "Float (single-precision)")))

(event `self.PawnSensing.OnSeePawn`
  (params (Pawn :type "Pawn Object Reference"))
  (if (and (`self.ActorHasTag` Pawn "Player") (not (`self.Alerted`)))
    (set `self.Alerted` true)
    (`|ExecutionSequence`
      (:`then_0`
        (bind _returnvalue (`AIBlueprintHelperLibrary.GetAIController` self))
        (bind _returnvalue_2 (`AIBlueprintHelperLibrary.GetBlackboard` _returnvalue))
        (`BlackboardComponent.SetValueAsBool` _returnvalue_2 (`self.AlertedKeyName`) true)
        (`BlackboardComponent.SetValueAsObject` _returnvalue_2 (`self.TargetKeyName`) Pawn))
      (:`then_1`
        (`AudioComponent.SetSound` (`self.HeavyBreathing`) "/Game/TwoButtons/Audio/Effects/Alerted.Alerted")))))

(fn `UserConstructionScript`)