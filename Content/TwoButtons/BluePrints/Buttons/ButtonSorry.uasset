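; ButtonSorry is a button that, when pressed, adds another monster but moves the player to safety and calms the threat.
; RecievePress spawns a BP_TheMonster running BT_Monster at a fixed location, then calls WarpPlayer and CalmEnemies.
; WarpPlayer moves the player to a random BP_SafeSpot transform.
; CalmEnemies clears Alerted on every monster and its blackboard, and resets its heavy-breathing sound.
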(event `self.ReceiveBeginPlay`)

(event `self.ReceiveActorBeginOverlap`
  (params (OtherActor :type "Actor Object Reference")))

(event `self.ReceiveTick`
  (params (DeltaSeconds :type "Float (single-precision)")))

(event `/Game/TwoButtons/BluePrints/Buttons/I_Button.RecievePress`
  (`AIBlueprintHelperLibrary.SpawnAIFromClass` "/Game/TwoButtons/BluePrints/Monster/BP_TheMonster.BP_TheMonster_C" "/Game/TwoButtons/BluePrints/Monster/AI/BT_Monster.BT_Monster" (590.0 140.0 390.0))
  (`self.WarpPlayer`)
  (`self.CalmEnemies`))

(fn `CalmEnemies`
  (bind _outactors (`GameplayStatics.GetAllActorsOfClass` "/Game/TwoButtons/BluePrints/Monster/BP_TheMonster.BP_TheMonster_C"))
  (for _array_element _outactors
    (`BlackboardComponent.SetValueAsBool` (`AIBlueprintHelperLibrary.GetBlackboard` _array_element) "Alerted" false)
    (set `/Game/TwoButtons/BluePrints/Monster/BP_TheMonster.Alerted` false _array_element)
    (`AudioComponent.SetSound` (`/Game/TwoButtons/BluePrints/Monster/BP_TheMonster.HeavyBreathing` _array_element) "/Game/TwoButtons/Audio/Effects/HeavyBreathing_01.HeavyBreathing_01")))

(fn `UserConstructionScript`
  (`parent.UserConstructionScript`))

(fn `WarpPlayer`
  (bind _outactors (`GameplayStatics.GetAllActorsOfClass` "/Game/TwoButtons/BluePrints/BP_SafeSpot.BP_SafeSpot_C"))
  (`self.K2_SetActorTransform` (`GameplayStatics.GetPlayerCharacter` 0) (`SceneComponent.K2_GetComponentToWorld` (`/Game/TwoButtons/BluePrints/BP_SafeSpot.DefaultSceneRoot` (`KismetArrayLibrary.Array_Get` _outactors (`KismetMathLibrary.RandomInteger` (`KismetArrayLibrary.Array_Length` _outactors))))) false false))