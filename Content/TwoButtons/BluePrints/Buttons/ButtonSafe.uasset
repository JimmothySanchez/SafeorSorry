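; ButtonSafe is the "Safe" button actor in the Safe or Sorry game, ending the game when pressed.
; RecievePress sets GameOver on GM_SafeOrSorry and replaces all on-screen widgets with Widget_SafeScreen.
; It then sets Alive to false on PC_SafeOrSorry and destroys the player character, even though this is the safe outcome.
; Construction defers to the parent class, and the other default events are unused.
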(event `self.ReceiveBeginPlay`)

(event `self.ReceiveActorBeginOverlap`
  (params (OtherActor :type "Actor Object Reference")))

(event `self.ReceiveTick`
  (params (DeltaSeconds :type "Float (single-precision)")))

(event `/Game/TwoButtons/BluePrints/Buttons/I_Button.RecievePress`
  (bind _returnvalue (`GameplayStatics.GetPlayerCharacter` 0))
  (bind _asgm_safe_or_sorry (cast `/Game/TwoButtons/BluePrints/GM_SafeOrSorry` (`GameplayStatics.GetGameMode`)))
  (set `/Game/TwoButtons/BluePrints/GM_SafeOrSorry.GameOver` true _asgm_safe_or_sorry)
  (bind _returnvalue_2 (`|CreateWidget` "/Game/TwoButtons/UIWidgets/Widget_SafeScreen.Widget_SafeScreen_C"))
  (`WidgetLayoutLibrary.RemoveAllWidgets`)
  (`UserWidget.AddToViewport` _returnvalue_2 0)
  (bind _aspc_safe_or_sorry (cast `/Game/TwoButtons/BluePrints/PC_SafeOrSorry` (`Pawn.GetController` _returnvalue)))
  (set `/Game/TwoButtons/BluePrints/PC_SafeOrSorry.Alive` false _aspc_safe_or_sorry)
  (`self.K2_DestroyActor` _returnvalue))

(fn `UserConstructionScript`
  (`parent.UserConstructionScript`))