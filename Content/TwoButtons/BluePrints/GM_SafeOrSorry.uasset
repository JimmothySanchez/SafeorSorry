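; GM_SafeOrSorry is a game mode that keeps score in a game where more live monsters earn more points.
; While the game is not over, Tick counts BP_TheMonster actors and calls UpdateScore at timed intervals, adding points that grow exponentially with that count.
; Each time the count exceeds its previous high, a flat bonus is added.
; Reset clears the score, timer, monster high mark and game-over flag.
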(event `self.ReceiveBeginPlay`)

(event `self.ReceiveTick`
  (params (DeltaSeconds :type "Float (single-precision)"))
  (if (not (`self.GameOver`))
    (`|ExecutionSequence`
      (:`then_0`
        (bind _outactors (`GameplayStatics.GetAllActorsOfClass` "/Game/TwoButtons/BluePrints/Monster/BP_TheMonster.BP_TheMonster_C"))
        (bind _returnvalue (`KismetArrayLibrary.Array_Length` _outactors))
        (if (> _returnvalue 0)
          (`|ExecutionSequence`
            (:`then_0`
              (set `self.TimeSinceScore` (+ (`self.TimeSinceScore`) DeltaSeconds)))
            (:`then_1`
              (if (> (`self.TimeSinceScore`) (`self.ScoreTimeIntervals`))
                (`self.UpdateScore` _returnvalue)
                (set `self.TimeSinceScore` 0.0))))))
      (:`then_1`
        (if (> _returnvalue (`self.PreviousMonsterCount`))
          (set `self.Score` (+ (`self.Score`) 1000))
          (set `self.PreviousMonsterCount` _returnvalue))))))

(fn `Reset`
  (set `self.GameOver` false)
  (set `self.PreviousMonsterCount` 0)
  (set `self.Score` 0)
  (set `self.TimeSinceScore` 0.0))

(fn `UpdateScore`
  (params (MonsterCount :type Integer))
  (set `self.Score` (`KismetMathLibrary.FTrunc` (+ (* (`KismetMathLibrary.MultiplyMultiply_FloatFloat` 2.0 (`KismetMathLibrary.Conv_IntToDouble` MonsterCount)) 10.0) (`KismetMathLibrary.Conv_IntToDouble` (`self.Score`))))))

(fn `UserConstructionScript`)