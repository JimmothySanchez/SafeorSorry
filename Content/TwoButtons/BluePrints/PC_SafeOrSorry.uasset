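; Player controller for the SafeOrSorry game mode that handles player death and restart.
; Die destroys the controlled pawn, swaps all widgets for the death screen, sets GameOver on the game mode and clears Alive.
; Releasing Jump while dead removes monsters, spawns and possesses a fresh first-person character at the first PlayerStart, restores the HUD and resets the game mode without reloading the level.
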(event `self.ReceiveBeginPlay`)

(event `self.ReceiveTick`
  (params (DeltaSeconds :type "Float (single-precision)")))

(event `InputAction|Jump` :consume false
  (params (Key :type "Key Structure" :default "AnyKey"))
  (:`Released`
    (if (not (`self.Alive`))
      (bind _outactors (`GameplayStatics.GetAllActorsOfClass` "/Game/TwoButtons/BluePrints/Monster/BP_TheMonster.BP_TheMonster_C"))
      (`self.K2_DestroyActor` _outactors)
      (bind _outactors_2 (`GameplayStatics.GetAllActorsOfClass` "/Script/Engine.PlayerStart"))
      (bind _returnvalue (`|SpawnActorFromClass` "/Game/TwoButtons/BluePrints/FirstPerson/FirstPersonCharacter.FirstPersonCharacter_C" (`self.GetTransform` (`KismetArrayLibrary.Array_Get` _outactors_2)) "AdjustIfPossibleButAlwaysSpawn" "OverrideRootScale"))
      (`self.Possess` _returnvalue)
      (`WidgetLayoutLibrary.RemoveAllWidgets`)
      (bind _returnvalue_2 (`|CreateWidget` "/Game/TwoButtons/UIWidgets/Widget_HUD.Widget_HUD_C"))
      (`UserWidget.AddToViewport` _returnvalue_2 0)
      (bind _asgm_safe_or_sorry (cast `/Game/TwoButtons/BluePrints/GM_SafeOrSorry` (`GameplayStatics.GetGameMode`)))
      (`/Game/TwoButtons/BluePrints/GM_SafeOrSorry.Reset` _asgm_safe_or_sorry)
      (set `self.Alive` true))))

(fn `Die`
  (`self.K2_DestroyActor` (`self.K2_GetPawn`))
  (`WidgetLayoutLibrary.RemoveAllWidgets`)
  (bind _returnvalue (`|CreateWidget` "/Game/TwoButtons/UIWidgets/Widget_Death.Widget_Death_C"))
  (`UserWidget.AddToViewport` _returnvalue 0)
  (bind _asgm_safe_or_sorry (cast `/Game/TwoButtons/BluePrints/GM_SafeOrSorry` (`GameplayStatics.GetGameMode`)))
  (set `/Game/TwoButtons/BluePrints/GM_SafeOrSorry.GameOver` true _asgm_safe_or_sorry)
  (set `self.Alive` false))

(fn `UserConstructionScript`)